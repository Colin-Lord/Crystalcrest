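; Player character for a top-down shooter, with movement, a roll montage, pistol and spread-shot shotgun, and a pause menu.
; Tick turns the mesh toward movement, feeds animation speed, detects mouse or gamepad input, regenerates health and toggles weapon visibility.
; WeaponArm aims at the cursor trace or right stick, while firing spawns bullet actors behind per-weapon cooldowns.
; Zero health triggers slow motion and an impulse-launched ragdoll; H debug-spawns enemies.
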(event `InputAction|Roll`
  (params (Key :type "Key Structure"))
  ;[1 1 1] Roll/Dodge
  (:`Pressed`
    (if (not (`NavMovementComponent.IsFalling` (`self.CharacterMovement`)))
      (`/Engine/EditorBlueprintResources/StandardMacros.DoOnce` false :!label _label
        (:`Completed`
          (`|PlayMontage` (`self.Mesh`) "/Game/Blueprints/Player/Animations/Roll/Roll_Anim_Montage.Roll_Anim_Montage"
            (:`OnCompleted`
              (goto _label :!via `Reset`))))))))

(event `InputAxis|WalkLeftRight`
  (params (AxisValue :type "Float (single-precision)"))
  ;[1 1 1] Movement
  (if (not (`self.Dying?`))
    (`self.AddMovementInput` (-1.0 1.0 0.0) AxisValue)))

(event `InputAxis|WalkForwardBack`
  (params (AxisValue :type "Float (single-precision)"))
  ;[1 1 1] Movement
  (if (not (`self.Dying?`))
    (`self.AddMovementInput` (1.0 1.0 0.0) AxisValue)))

(event `self.ReceiveTick`
  (params (DeltaSeconds :type "Float (single-precision)"))
  (bind _returnvalue (`GameplayStatics.GetPlayerController` 0))
  (bind _mesh (`self.Mesh`))
  (bind _currentinputmouseorkeyboard (`self.CurrentInputMouseOrKeyboard`))
  (bind _playerhealth (`self.PlayerHealth`))
  (bind _weaponarm (`self.WeaponArm`))
  (bind _currentweapon (`self.CurrentWeapon`))
  (bind _shotgun (`self.Shotgun`))
  (bind _gun (`self.Gun`))
  (bind _shotgun_2 (`self.Shotgun`))
  (bind _gun_2 (`self.Gun`))
  (bind (_returnvalue_roll _returnvalue_pitch) (`KismetMathLibrary.BreakRotator` (`SceneComponent.K2_GetComponentRotation` _weaponarm)))
  (bind _returnvalue_2 (`CharacterMovementComponent.GetCurrentAcceleration` (`self.CharacterMovement`)))
  (bind (_bblockinghit _binitialoverlap _time _distance _location) (`GameplayStatics.BreakHitResult` (`PlayerController.GetHitResultUnderCursorByChannel` (`GameplayStatics.GetPlayerController` 0) "TraceTypeQuery1" true)))
  (bind (_returnvalue_roll_2 _returnvalue_pitch_2 _returnvalue_yaw) (`KismetMathLibrary.BreakRotator` (`KismetMathLibrary.Conv_VectorToRotator` _returnvalue_2)))
  (bind (_returnvalue_roll_3 _returnvalue_pitch_3 _returnvalue_yaw_2) (`KismetMathLibrary.BreakRotator` (`KismetMathLibrary.FindLookAtRotation` (`SceneComponent.K2_GetComponentLocation` _weaponarm) _location)))
  ;[1 1 1] Rotates gun towards mouse cursor
  (`|ExecutionSequence`
    (:`then_0`
      ;[1 1 1] Rotates Player Towards Movement
      (if (!= _returnvalue_2 (0.0 0.0 0.0))
        (`SceneComponent.K2_SetWorldRotation` _mesh (`KismetMathLibrary.RInterpTo` (`SceneComponent.K2_GetComponentRotation` _mesh) (`KismetMathLibrary.MakeRotator` 0.0 0.0 (+ _returnvalue_yaw -90.0)) 1.0 0.1) false false)))
    (:`then_1`
      ;[1 1 1] Updates Animation Speed Variable
      (bind _asplayer_anim_bp (cast `/Game/Blueprints/Player/Animations/PlayerAnimBP` (`SkeletalMeshComponent.GetAnimInstance` (`self.Mesh`))))
      (set `/Game/Blueprints/Player/Animations/PlayerAnimBP.Speed` (`KismetMathLibrary.VSizeSquared` (`self.GetVelocity`)) _asplayer_anim_bp))
    (:`then_2`
      (if _bblockinghit
        (if (`self.CurrentInputMouseOrKeyboard`)
          (if (not (`self.Dying?`))
            (`SceneComponent.K2_SetWorldRotation` (`self.WeaponArm`) (`KismetMathLibrary.MakeRotator` _returnvalue_roll _returnvalue_pitch (+ _returnvalue_yaw_2 180.0)) false true)))))
    (:`then_3`
      ;[1 1 1] Determines whether current input is mouse keyboard or controller
      (if (or (!= (`self.GetInputAxisKeyValue`) 0.0) (!= (`self.GetInputAxisKeyValue`) 0.0))
        (set `self.CurrentInputMouseOrKeyboard` true)
        (elif (or (!= (`self.GetInputAxisKeyValue`) 0.0) (!= (`self.GetInputAxisKeyValue`) 0.0) (!= (`self.GetInputAxisKeyValue`) 0.0) (!= (`self.GetInputAxisKeyValue`) 0.0) (!= (`self.GetInputAxisKeyValue`) 0.0) (!= (`self.GetInputAxisKeyValue`) 0.0))
          (set `self.CurrentInputMouseOrKeyboard` false))))
    (:`then_4`
      ;[1 1 1] Hides Mouse Cursor If the input mode is controller
      (set `PlayerController.bShowMouseCursor` _currentinputmouseorkeyboard _returnvalue)
      (if (not _currentinputmouseorkeyboard)
        (`PlayerController.SetMouseLocation` _returnvalue 960 540)))
    (:`then_5`
      ;[1 1 1] RecieveDamage
      (if (not (`self.Dying?`))
        (bind _ashealth_ui (cast `/Game/Blueprints/UI/HealthUI` (`WidgetComponent.GetUserWidgetObject` (`self.Widget`))))
        (if (not (>= _playerhealth 100.0))
          (set `/Game/Blueprints/UI/HealthUI.Health` _playerhealth _ashealth_ui)
          (set `self.PlayerHealth` (+ (`self.PlayerHealth`) 0.05)))))
    (:`then_6`
      ;[1 1 1] Death/Ragdoll
      (if (<= (`self.PlayerHealth`) 0.0)
        (`GameplayStatics.SetGlobalTimeDilation` 0.4)
        (set `self.Dying?` true)
        (`/Engine/EditorBlueprintResources/StandardMacros.DoOnce` false
          (:`Completed`
            (`PrimitiveComponent.SetSimulatePhysics` (`self.Mesh`) true)
            (`CharacterMovementComponent.DisableMovement` (`self.CharacterMovement`))
            (`ActorComponent.K2_DestroyComponent` (`self.WeaponArm`))
            (`ActorComponent.K2_DestroyComponent` (`self.Gun`))
            (`ActorComponent.K2_DestroyComponent` (`self.BulletAimer`))
            (`ActorComponent.K2_DestroyComponent` (`self.Widget`))
            (`PrimitiveComponent.AddImpulse` (`self.Mesh`) (`KismetMathLibrary.MakeVector` (`KismetMathLibrary.RandomFloatInRange` -1000.0 1000.0) (`KismetMathLibrary.RandomFloatInRange` -1000.0 1000.0) 1000.0) "None" true)))))
    (:`then_7`
      (if (== _currentweapon 1)
        (`/Engine/EditorBlueprintResources/StandardMacros.IsValid` _shotgun_2
          (:`Is Valid`
            (`SceneComponent.SetVisibility` _shotgun_2 false false)
            (`/Engine/EditorBlueprintResources/StandardMacros.IsValid` _gun
              (:`Is Valid`
                (`SceneComponent.SetVisibility` _gun true false)))))
        (elif (== _currentweapon 2)
          (`/Engine/EditorBlueprintResources/StandardMacros.IsValid` _gun_2
            (:`Is Valid`
              (`SceneComponent.SetVisibility` _gun_2 false false)
              (`/Engine/EditorBlueprintResources/StandardMacros.IsValid` _shotgun
                (:`Is Valid`
                  (`SceneComponent.SetVisibility` _shotgun true false))))))))))

(event `self.ReceiveAnyDamage`
  (params (Damage :type "Float (single-precision)") (DamageType :type "DamageType Object Reference") (InstigatedBy :type "Controller Object Reference") (DamageCauser :type "Actor Object Reference"))
  ;[1 1 1] RecieveDamage
  (set `self.PlayerHealth` (- (`self.PlayerHealth`) Damage)))

(event `InputAction|ChangeWeaponUp`
  (params (Key :type "Key Structure"))
  (bind _currentweapon (`self.CurrentWeapon`))
  (:`Pressed`
    (if (not (== _currentweapon 2))
      (set `self.CurrentWeapon` (+ _currentweapon 1)))))

(event `InputAction|ChangeWeaponDown`
  (params (Key :type "Key Structure"))
  (bind _currentweapon (`self.CurrentWeapon`))
  (:`Pressed`
    (if (not (== _currentweapon 1))
      (set `self.CurrentWeapon` (+ _currentweapon -1)))))

(event `self.ReceiveBeginPlay`
  ;[1 1 1] Starts the health bar at 100%
  (`|ExecutionSequence`
    (:`then_0`
      (bind _ashealth_ui (cast `/Game/Blueprints/UI/HealthUI` (`WidgetComponent.GetUserWidgetObject` (`self.Widget`))))
      (set `/Game/Blueprints/UI/HealthUI.Health` (`self.PlayerHealth`) _ashealth_ui))))

(event `Key|H`
  (params (Key :type "Key Structure"))
  ;[1 1 1] Debugging Enemy Ai
  (:`Pressed`
    (`|SpawnActorFromClass` "/Game/Blueprints/EnemyAI/EnemyAI/EnemyCharacterBP.EnemyCharacterBP_C" (`KismetMathLibrary.MakeTransform` (`.Location` (`GameplayStatics.BreakHitResult` (`PlayerController.GetHitResultUnderCursorByChannel` (`GameplayStatics.GetPlayerController` 0) "TraceTypeQuery1" true)))) "Undefined" "OverrideRootScale" null null)))

(event `InputAction|SetWeapon1`
  (params (Key :type "Key Structure"))
  (:`Pressed`
    (set `self.CurrentWeapon` 1)))

(event `InputAction|SetWeapon2`
  (params (Key :type "Key Structure"))
  (:`Pressed`
    (set `self.CurrentWeapon` 2)))

(event `InputAction|FireGun`
  (params (Key :type "Key Structure"))
  (bind _bulletaimer (`self.BulletAimer`))
  (bind _bulletaimer_2 (`self.BulletAimer`))
  (bind _bulletaimer_3 (`self.BulletAimer`))
  (bind _currentweapon (`self.CurrentWeapon`))
  (bind (_returnvalue_roll _returnvalue_pitch _returnvalue_yaw) (`KismetMathLibrary.BreakRotator` (`SceneComponent.K2_GetComponentRotation` _bulletaimer)))
  (bind (_returnvalue_roll_2 _returnvalue_pitch_2 _returnvalue_yaw_2) (`KismetMathLibrary.BreakRotator` (`SceneComponent.K2_GetComponentRotation` _bulletaimer_2)))
  (bind (_returnvalue_roll_3 _returnvalue_pitch_3 _returnvalue_yaw_3) (`KismetMathLibrary.BreakRotator` (`SceneComponent.K2_GetComponentRotation` _bulletaimer_3)))
  ;[1 1 1] Gun Animation, Particles and Bullets
  (:`Pressed`
    (if (`self.Dying?`)
      _
      (elif (== _currentweapon 1)
        ;;[1 1 1] Pistol Gun
        (if (not (`self.PistolGunCooldown?`))
          (set `self.PistolGunCooldown?` true)
          (`|SpawnActorFromClass` "/Game/Blueprints/Bullets/PistolBullet.PistolBullet_C" (`KismetMathLibrary.MakeTransform` (`SceneComponent.K2_GetComponentLocation` (`self.BulletAimer`)) (`SceneComponent.K2_GetComponentRotation` (`self.Gun`)) (0.1 0.1 0.1)) "Undefined" "OverrideRootScale" null null)
          (`SkeletalMeshComponent.PlayAnimation` (`self.Gun`) "/Game/Blueprints/Player/Weapons/Pistol/PistolShoot_Anim.PistolShoot_Anim" false)
          (`NiagaraFunctionLibrary.SpawnSystemAtLocation` "/Game/Blueprints/Particles/GunParticleSystem.GunParticleSystem" (`SceneComponent.K2_GetComponentLocation` _bulletaimer) (`KismetMathLibrary.MakeRotator` _returnvalue_roll _returnvalue_pitch (+ _returnvalue_yaw 180.0)))
          (if (not (`self.CurrentInputMouseOrKeyboard`))
            (`GameplayStatics.SpawnForceFeedbackAttached` "/Game/Blueprints/ControllerFeedback/ShootFeedback.ShootFeedback" (`self.BulletAimer`) "None" (0.0 0.0 0.0) (struct) "KeepRelativeOffset" false false 1.0 0.0 null))
          (`KismetSystemLibrary.Delay` (`self.PistolGunCooldown`))
          (set `self.PistolGunCooldown?` false))
        (elif (== _currentweapon 2)
          ;;[1 1 1] Shotgun
          (if (not (`self.ShotgunCooldown?`))
            (set `self.ShotgunCooldown?` true)
            (for _index (range 1 11)
              (`|SpawnActorFromClass` "/Game/Blueprints/Bullets/ShotgunBullet.ShotgunBullet_C" (`KismetMathLibrary.MakeTransform` (`SceneComponent.K2_GetComponentLocation` _bulletaimer_3) (`KismetMathLibrary.MakeRotator` 0.0 0.0 (+ _returnvalue_yaw_3 (- (* _index 10.0) 50.0))) (0.1 0.1 0.1)) "AlwaysSpawn" "OverrideRootScale" null null))
            (`SkeletalMeshComponent.PlayAnimation` (`self.Shotgun`) "/Game/Blueprints/Player/Weapons/Shotgun/ShotgunShoot_Anim.ShotgunShoot_Anim" false)
            (`NiagaraFunctionLibrary.SpawnSystemAtLocation` "/Game/Blueprints/Particles/GunParticleSystem.GunParticleSystem" (`SceneComponent.K2_GetComponentLocation` _bulletaimer_2) (`KismetMathLibrary.MakeRotator` _returnvalue_roll_2 _returnvalue_pitch_2 (+ _returnvalue_yaw_2 180.0)))
            (if (not (`self.CurrentInputMouseOrKeyboard`))
              (`GameplayStatics.SpawnForceFeedbackAttached` "/Game/Blueprints/ControllerFeedback/ShootFeedback.ShootFeedback" (`self.BulletAimer`) "None" (0.0 0.0 0.0) (struct) "KeepRelativeOffset" false false 1.0 0.0 null))
            (`KismetSystemLibrary.Delay` (`self.ShotgunCooldown`))
            (set `self.ShotgunCooldown?` false)))))))

(event `InputAxisKey|Gamepad_RightX`
  (params (AxisValue :type "Float (single-precision)"))
  (bind _weaponarm (`self.WeaponArm`))
  (bind _returnvalue (`SceneComponent.K2_GetComponentLocation` _weaponarm))
  ;[1 1 1] Controller Aiming
  (if (not (== (+ AxisValue (stale `InputAxisKey|Gamepad_RightY` AxisValue)) 0.0)) :!label _label_2
    (bind (_returnvalue_roll _returnvalue_pitch _returnvalue_yaw) (`KismetMathLibrary.BreakRotator` (`KismetMathLibrary.FindLookAtRotation` _returnvalue (+ _returnvalue (`KismetMathLibrary.MakeVector` AxisValue (stale `InputAxisKey|Gamepad_RightY` AxisValue))))))
    (`SceneComponent.K2_SetWorldRotation` _weaponarm (`KismetMathLibrary.MakeRotator` 0.0 0.0 (+ _returnvalue_yaw 135.0)) false false)))

(event `InputAxisKey|Gamepad_RightY`
  (params (AxisValue :type "Float (single-precision)"))
  ;[1 1 1] Controller Aiming
  (goto _label_2))

(event `Key|Tab`
  (params (Key :type "Key Structure"))
  (:`Pressed`
    (bind _returnvalue (`|CreateWidget` "/Game/Blueprints/UI/PauseMenu/PauseMenuUI.PauseMenuUI_C"))
    (`UserWidget.AddToViewport` _returnvalue 0)))

(fn `UserConstructionScript`)